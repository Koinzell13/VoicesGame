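; Spatialized music stem actor that plays one sound through a granular synth and visualizes its loudness, with configurable attenuation, bus and submix routing.
; While a gate is open, Tick drives the playhead from elapsed time and applies pitch, grain duration and density controls, decoupling pitch from playback position.
; At the sound's end the gate restarts or closes.
; The envelope follower stretches a cylinder's height, normalized against a slowly decaying peak to stay responsive.
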(event `self.ReceiveBeginPlay`
  ;[1 1 1] beginPlay
  (set `self.startingRelScale` (`self.GetActorRelativeScale3D`))
  ;[1 1 1] boot up granular
  (`|ExecutionSequence`
    (:`then_0`
      (`/Game/ArthursAudioBPs/Core/FunctionLibraries/AabpsGranularSynthHelpers.UpdateFullGranularPreset` (`self.GranularSynth`) (`self.GranularPresetBase`)))
    (:`then_1`
      (`GranularSynth.SetSoundWave` (`self.GranularSynth`) (`self.Sound`)))
    (:`then_2`
      (`KismetSystemLibrary.Delay` 0.2)
      (`/Game/ArthursAudioBPs/Core/FunctionLibraries/AabpsGranularSynthHelpers.StartGranular` (`self.GranularSynth`))
      ;[1 1 1] Open gate
      (`self.OpenGate`))
    (:`then_3`
      ;[1 1 1] increase volume viz sensitivity
      (`KismetSystemLibrary.K2_SetTimerDelegate` (delegate `DecreaseMaxVolRegistered`) 0.25 true))))

(event `self.ReceiveTick`
  (params (DeltaSeconds :type "Float (single-precision)"))
  ;[1 1 1] tick
  (bind _output_get (set `self.ActorElapsedTime` (+ (stale _output_get) DeltaSeconds)))
  ;[1 1 1] gate
  (`/Engine/EditorBlueprintResources/StandardMacros.Gate` true :!label _label
    (:`Exit`
      ;[1 1 1] store latest elapsed time
      (set `self.LatestElapsedTime` (- (`self.ActorElapsedTime`) (`self.StartTime`)))
      ;[1 1 1] gone through sample?
      (if (>= (`self.LatestElapsedTime`) (`SoundBase.Duration` (`self.Sound`)))
        ;[1 1 1] Finished
        ;;[1 1 1] loop?
        (if (`self.Loop`)
          ;;[1 1 1] Open Gate
          (`self.OpenGate`)
          (else
            ;;[1 1 1] close gate
            (`self.CloseGate`)))
        (else
          ;[1 1 1] Still playing
          ;;[1 1 1] update pitch
          (`GranularSynth.SetGrainPitch` (`self.GranularSynth`) (`self.PitchMP`) (0.0 0.0))
          ;;[1 1 1] update playhead time
          (`GranularSynth.SetPlayheadTime` (`self.GranularSynth`) (`self.LatestElapsedTime`) 0.0 "FromBeginning")
          ;;[1 1 1] grain duration
          (`GranularSynth.SetGrainDuration` (`self.GranularSynth`) (* (* (`.DurationBaseMsec_55_629930E44F1507F01122F697D24D492F` (break `/Game/ArthursAudioBPs/Core/FunctionLibraries/AabpsGranularPreset` (`self.GranularPresetBase`))) (`self.GrainDurationMP_0`)) (`self.GrainDurationMP_1`)) (0.0 0.0))
          ;;[1 1 1] grainsPerSecond
          (`GranularSynth.SetGrainsPerSecond` (`self.GranularSynth`) (* (`.GrainsPerSecond_28_FB913A6443DB4978747958AE9B07E7B1` (break `/Game/ArthursAudioBPs/Core/FunctionLibraries/AabpsGranularPreset` (`self.GranularPresetBase`))) (`self.GrainsPerSecond`))))))))

(event `DecreaseMaxVolRegistered`
  ;[1 1 1] increase volume viz sensitivity
  (bind _output_get (set `self.MaxEnvelope` (* (stale _output_get) 0.95))))

(event `OpenGate`
  ;[1 1 1] gate
  ;;[1 1 1] store current time
  (set `self.StartTime` (`self.ActorElapsedTime`))
  (goto _label :!via `Open`))

(event `CloseGate`
  ;[1 1 1] gate
  (goto _label :!via `Close`))

(event `self.GranularSynth.OnAudioEnvelopeValue`
  (params (EnvelopeValue :type "Float (single-precision)"))
  ;[1 1 1] Envelope/volume
  (bind _output_get (set `self.LatestEnvelope` EnvelopeValue))
  (if (> _output_get (stale _output_get_2))
    (bind _output_get_2 (set `self.MaxEnvelope` _output_get)))
  (set `self.currentVolume` (`KismetMathLibrary.MapRangeClamped` (`self.LatestEnvelope`) 0.0 (`self.MaxEnvelope`) 0.0 1.0))
  ;[1 1 1] change mesh scale
  (`SceneComponent.SetRelativeScale3D` (`self.Cylinder`) (`KismetMathLibrary.MakeVector` (.x (`self.startingRelScale`)) (.y (`self.startingRelScale`)) (* (.z (`self.startingRelScale`)) (+ (* (`self.currentVolume`) 5.0) 0.5)))))

(fn `UserConstructionScript`
  ;[1 1 1] attenuation
  (set `SynthComponent.AttenuationSettings` (`self.Attenuation`) (`self.GranularSynth`))
  ;[1 1 1] bus sends
  (`SynthComponent.SetOutputToBusOnly` (`self.GranularSynth`) (`self.OutputToBusOnly`))
  (set `SynthComponent.PreEffectBusSends` (`self.Pre-Effect Bus Sends`) (`self.GranularSynth`))
  (set `SynthComponent.BusSends` (`self.Post-EffectSourceBusSends`) (`self.GranularSynth`))
  ;[1 1 1] submix sends
  (for _array_element (`self.SubmixSends`)
    (`SynthComponent.SetSubmixSend` (`self.GranularSynth`) _array_element 1.0))
  ;[1 1 1] envelope attack/rls
  (set `SynthComponent.EnvelopeFollowerAttackTime` (`self.Attack`) (`self.GranularSynth`))
  (set `SynthComponent.EnvelopeFollowerReleaseTime` (`self.Release`) (`self.GranularSynth`)))