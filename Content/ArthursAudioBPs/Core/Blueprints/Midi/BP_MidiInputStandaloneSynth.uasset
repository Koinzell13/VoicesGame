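; Standalone MIDI-driven synth Blueprint that plays a modular synth component from the default MIDI input device.
; On BeginPlay it creates a MIDI input controller, binds its events and applies the synth preset.
; Note on/off events drive the synth directly, while pitch bend is scaled to a configurable semitone range.
; Mod wheel control change on channel 1 maps to release time, and note-on and control change events print debug strings.
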(event `self.ReceiveBeginPlay`
  ;[1 1 1] set up default midi device
  (bind _deviceid (`MIDIDeviceManager.GetDefaultMIDIInputDeviceID`))
  (bind _returnvalue (`MIDIDeviceManager.CreateMIDIDeviceInputController` _deviceid))
  (bind _output_get (set `self.MidiController` _returnvalue))
  ;[1 1 1] set up midi events
  (add `MIDIDeviceInputController.OnMIDINoteOn` _output_get (delegate `OnMIDINoteOn_Event_0`))
  (add `MIDIDeviceInputController.OnMIDINoteOff` _output_get (delegate `OnMIDINoteOff_Event_0`))
  (add `MIDIDeviceInputController.OnMIDIPitchBend` _output_get (delegate `OnMIDIPitchBend_Event_0`))
  (add `MIDIDeviceInputController.OnMIDIControlChange` _output_get (delegate `OnMIDIControlChange_Event_0`))
  ;[1 1 1] set up synth component
  (`ModularSynthComponent.SetSynthPreset` (`self.ModularSynth`) (`self.SynthPreset`)))

(event `OnMIDINoteOn_Event_0`
  (params (MIDIDeviceController :type "MIDIDeviceInputController Object Reference") (Timestamp :type Integer) (Channel :type Integer) (Note :type Integer) (Velocity :type Integer))
  ;[1 1 1] midi events
  ;[1 1 1] note on
  (`KismetSystemLibrary.PrintString` (`KismetStringLibrary.Concat_StrStr` "Note: " (`KismetStringLibrary.Conv_IntToString` Note) " Velocity: " (`KismetStringLibrary.Conv_IntToString` Velocity)))
  (`ModularSynthComponent.NoteOn` (`self.ModularSynth`) (`KismetMathLibrary.Conv_IntToDouble` Note) Velocity -1.0))

(event `OnMIDINoteOff_Event_0`
  (params (MIDIDeviceController :type "MIDIDeviceInputController Object Reference") (Timestamp :type Integer) (Channel :type Integer) (Note :type Integer) (Velocity :type Integer))
  ;[1 1 1] midi events
  ;[1 1 1] note off
  (`ModularSynthComponent.NoteOff` (`self.ModularSynth`) (`KismetMathLibrary.Conv_IntToDouble` Note) false false))

(event `OnMIDIPitchBend_Event_0`
  (params (MIDIDeviceController :type "MIDIDeviceInputController Object Reference") (Timestamp :type Integer) (Channel :type Integer) (Pitch :type Integer))
  (bind _pitchbendrangeinsemitones (`self.PitchBendRangeInSemitones`))
  ;[1 1 1] midi events
  ;[1 1 1] pitch bend
  (`ModularSynthComponent.SetPitchBend` (`self.ModularSynth`) (`KismetMathLibrary.MapRangeUnclamped` (`KismetMathLibrary.Conv_IntToDouble` Pitch) 0.0 16384.0 (* _pitchbendrangeinsemitones -1.0) _pitchbendrangeinsemitones)))

(event `OnMIDIControlChange_Event_0`
  (params (MIDIDeviceController :type "MIDIDeviceInputController Object Reference") (Timestamp :type Integer) (Channel :type Integer) (Type :type Integer) (Value :type Integer))
  ;[1 1 1] midi events
  ;[1 1 1] print midi control change
  (`KismetSystemLibrary.PrintString` (`KismetStringLibrary.Concat_StrStr` "channel: " (`KismetStringLibrary.Conv_IntToString` Channel) " \nType: " (`KismetStringLibrary.Conv_IntToString` Type) " \nValue: " (`KismetStringLibrary.Conv_IntToString` Value)))
  ;[1 1 1] map mod wheel to release time (well channel 1/type 1 at least, thats mod wheel channel on my midi controller)
  (if (and (== Channel 1) (== Type 1))
    (`ModularSynthComponent.SetReleaseTime` (`self.ModularSynth`) (`KismetMathLibrary.MapRangeClamped` (`KismetMathLibrary.Conv_IntToDouble` Value) 0.0 127.0 5.0 5000.0))))

(fn `UserConstructionScript`)